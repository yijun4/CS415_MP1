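; BP_Bullet is a projectile that flies along world X and disappears when it hits the tunnel.
; Each tick it moves by a swept world offset, then sets its speed to the referenced player's forward speed plus a fixed margin, so it stays ahead of the player.
; An overlap on its Bullet component with a BP_Tunnel destroys it; other actors are ignored.
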(event OnComponentBeginOverlap(bullet)
  (params (OverlappedComponent :type Primitive%20Component%20Object%20Reference) (OtherActor :type Actor%20Object%20Reference) (OtherComp :type Primitive%20Component%20Object%20Reference) (OtherBodyIndex :type Integer) (bFromSweep :type Boolean) (SweepResult :type Hit%20Result%20Structure%20%28by%20ref%29))
  (Utilities|Casting|CastToBP_Tunnel OtherActor)
  (Utilities|FlowControl|Sequence
    (:then_0
      (Actor|DestroyActor))))

(event EventTick
  (params (DeltaSeconds :type Float%20%28single-precision%29))
  (Transformation|AddActorWorldOffset (Math|Vector|MakeVector (* DeltaSeconds (Variables|Default|GetShoot%20Speed)) 0.0 0.0) true)
  (Variables|Default|SetShoot%20Speed (+ (Variables|/Game/InfiniteMatrix/Blueprints/BP_Player.BP_Player_C|GetForwardSpeed (Variables|Default|Getcurrplayer)) 2.5e+03)))

(fn ConstructionScript)